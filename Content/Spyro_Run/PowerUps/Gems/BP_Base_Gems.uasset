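; Base gem pickup for the Spyro runner, collected when the player character overlaps its sphere.
; It finds the GemManager at BeginPlay, then on pickup plays a sound and adds its gem value to that manager.
; It broadcasts CollectGemMessage to every widget and actor implementing the BI_Runner interface, then destroys itself.
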(event OnComponentBeginOverlap(Sphere)
  (params (OverlappedComponent :type Primitive%20Component%20Object%20Reference) (OtherActor :type Actor%20Object%20Reference) (OtherComp :type Primitive%20Component%20Object%20Reference) (OtherBodyIndex :type Integer) (bFromSweep :type Boolean) (SweepResult :type Hit%20Result%20Structure%20%28by%20ref%29))
  (if (== OtherActor (Game|GetPlayerCharacter 0))
    (Audio|PlaySound2D (Variables|Default|GetPickup%20Sound))
    (Default|AddGems (Variables|Default|GetGemManager) (Variables|Default|GetGemValue))
    (Utilities|FlowControl|Sequence
      (:then_0
        (bind _foundwidgets (Class|WidgetBlueprintLibrary|GetAllWidgetswithInterface "/Game/Spyro_Run/BI_Runner.BI_Runner_C" false))
        (for _array_element _foundwidgets
          (Class|BIRunner|CollectGem(Message) _array_element)))
      (:then_1
        (bind _outactors (Actor|GetAllActorswithInterface "/Game/Spyro_Run/BI_Runner.BI_Runner_C"))
        (for _array_element_2 _outactors
          (Class|BIRunner|CollectGem(Message) _array_element_2)))
      (:then_2
        (Actor|DestroyActor)))))

(event EventBeginPlay
  (bind _outactors (Actor|GetAllActorsOfClass "/Game/Spyro_Run/PowerUps/GemManager.GemManager_C"))
  (Variables|Default|SetGemManager (Utilities|Array|Get(acopy) _outactors)))

(fn ConstructionScript)