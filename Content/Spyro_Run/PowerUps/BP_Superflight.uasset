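; BP_Superflight is a Spyro runner power-up pickup that grants the player ten seconds of flight.
; On player overlap it hides its mesh and, if the PowerupManager has no active power-up, claims that flag; otherwise it destroys itself without effect.
; While active it loops the fly montage and pins the player's height each Tick, then stops the montage, clears the flag and destroys itself.
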(event OnComponentBeginOverlap(Sphere)
  (params (OverlappedComponent :type Primitive%20Component%20Object%20Reference) (OtherActor :type Actor%20Object%20Reference) (OtherComp :type Primitive%20Component%20Object%20Reference) (OtherBodyIndex :type Integer) (bFromSweep :type Boolean) (SweepResult :type Hit%20Result%20Structure%20%28by%20ref%29))
  (if (== OtherActor (Game|GetPlayerCharacter 0))
    (if (not (Variables|/Game/Spyro_Run/PowerUps/PowerupManager.PowerupManager_C|GetHasPowerup? (Variables|Default|GetPowerupManager)))
      (Rendering|SetVisibility (Variables|Default|GetStaticMesh) false false)
      (Variables|/Game/Spyro_Run/PowerUps/PowerupManager.PowerupManager_C|SetHasPowerup? (Variables|Default|GetPowerupManager) true)
      (CallFunction|ActivatePowerup)
      (else
        (Rendering|SetVisibility (Variables|Default|GetStaticMesh) false false)
        (Actor|DestroyActor)))))

(event Custom|ActivatePowerup
  (bind _returnvalue (Game|GetPlayerCharacter 0))
  (Variables|Default|SetPickedUp? true)
  (Animation|PlayAnimMontage _returnvalue "/CPS1999_Spyro/Animations/Montages/AM_CPS1999_Fly_Loop.AM_CPS1999_Fly_Loop" 1.0 "None")
  (Utilities|FlowControl|Delay 1e+01)
  (Animation|StopAnimMontage _returnvalue "/CPS1999_Spyro/Animations/Montages/AM_CPS1999_Fly_Loop.AM_CPS1999_Fly_Loop")
  (Variables|Default|SetPickedUp? false)
  (Variables|/Game/Spyro_Run/PowerUps/PowerupManager.PowerupManager_C|SetHasPowerup? (Variables|Default|GetPowerupManager) false)
  (Actor|DestroyActor))

(event EventBeginPlay
  (bind _outactors (Actor|GetAllActorsOfClass "/Game/Spyro_Run/PowerUps/PowerupManager.PowerupManager_C"))
  (bind _aspowerup_manager (Utilities|Casting|CastToPowerupManager (Utilities|Array|Get(acopy) _outactors)))
  (Variables|Default|SetPowerupManager _aspowerup_manager))

(event EventTick
  (params (DeltaSeconds :type Float%20%28single-precision%29))
  (bind _returnvalue (Game|GetPlayerCharacter 0))
  (bind _returnvalue_2 (Transformation|GetActorLocation _returnvalue))
  (if (Variables|Default|GetPickedUp?)
    (Transformation|SetActorLocation _returnvalue (Math|Vector|MakeVector (.x _returnvalue_2) (.y _returnvalue_2) 146.649994) false false)))

(fn ConstructionScript)