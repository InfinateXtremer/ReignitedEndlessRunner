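; Supercharge pickup that puts the player into flying mode with a supercharge material for about ten seconds.
; On overlap it claims the shared PowerupManager's HasPowerup flag, or destroys itself if another powerup is active.
; A Delay chain blinks the material before expiry, then restores walking and original speed and destroys the actor.
; Tick raises walk speed while PickedUp, but that flag is only set as the effect ends.
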(event OnComponentBeginOverlap(Sphere)
  (params (OverlappedComponent :type Primitive%20Component%20Object%20Reference) (OtherActor :type Actor%20Object%20Reference) (OtherComp :type Primitive%20Component%20Object%20Reference) (OtherBodyIndex :type Integer) (bFromSweep :type Boolean) (SweepResult :type Hit%20Result%20Structure%20%28by%20ref%29))
  (if (== OtherActor (Game|GetPlayerCharacter 0))
    (if (not (Variables|/Game/Spyro_Run/PowerUps/PowerupManager.PowerupManager_C|GetHasPowerup? (Variables|Default|GetPowerupManager)))
      (Rendering|SetVisibility (Variables|Default|GetStaticMesh) false false)
      (CallFunction|ActivatePowerup)
      (Variables|/Game/Spyro_Run/PowerUps/PowerupManager.PowerupManager_C|SetHasPowerup? (Variables|Default|GetPowerupManager) true)
      (Variables|Default|SetOriginalSpeed (Variables|/Script/Engine.CharacterMovementComponent|GetMaxWalkSpeed (Variables|/Script/Engine.Character|GetCharacterMovement (Game|GetPlayerCharacter 0))))
      (else
        (Actor|DestroyActor)))))

(event Custom|ActivatePowerup
  (bind _returnvalue (Game|GetPlayerCharacter 0))
  (bind _returnvalue_2 (Game|GetPlayerCharacter 0))
  (bind _charactermovement (Variables|/Script/Engine.Character|GetCharacterMovement _returnvalue))
  (bind _mesh (Variables|/Script/Engine.Character|GetMesh _returnvalue_2))
  (Pawn|Components|CharacterMovement|SetMovementMode (Variables|/Script/Engine.Character|GetCharacterMovement (Game|GetPlayerCharacter 0)) "MOVE_Flying" 0)
  (Rendering|Material|SetMaterial (Variables|/Script/Engine.Character|GetMesh (Game|GetPlayerCharacter 0)) 0 "/CPS1999_Spyro/Materials/MI_CPS1999_Spyro_SuperCharge.MI_CPS1999_Spyro_SuperCharge")
  (Utilities|FlowControl|Delay 6.0)
  (Rendering|Material|SetMaterial _mesh 0 "/CPS1999_Spyro/Mesh/ReferenceSpyro/MI_CPS1999_Spyro_Body.MI_CPS1999_Spyro_Body")
  (Utilities|FlowControl|Delay 1.0)
  (Rendering|Material|SetMaterial _mesh 0 "/CPS1999_Spyro/Materials/MI_CPS1999_Spyro_SuperCharge.MI_CPS1999_Spyro_SuperCharge")
  (Utilities|FlowControl|Delay 1.0)
  (Rendering|Material|SetMaterial _mesh 0 "/CPS1999_Spyro/Mesh/ReferenceSpyro/MI_CPS1999_Spyro_Body.MI_CPS1999_Spyro_Body")
  (Utilities|FlowControl|Delay 1.0)
  (Rendering|Material|SetMaterial _mesh 0 "/CPS1999_Spyro/Materials/MI_CPS1999_Spyro_SuperCharge.MI_CPS1999_Spyro_SuperCharge")
  (Utilities|FlowControl|Delay 1.0)
  (Rendering|Material|SetMaterial _mesh 0 "/CPS1999_Spyro/Mesh/ReferenceSpyro/MI_CPS1999_Spyro_Body.MI_CPS1999_Spyro_Body")
  (Variables|Default|SetPickedUp? true)
  (Variables|/Script/Engine.CharacterMovementComponent|SetMaxWalkSpeed _charactermovement (Variables|Default|GetOriginalSpeed))
  (Pawn|Components|CharacterMovement|SetMovementMode _charactermovement "MOVE_Walking" 0)
  (Variables|/Game/Spyro_Run/PowerUps/PowerupManager.PowerupManager_C|SetHasPowerup? (Variables|Default|GetPowerupManager) false)
  (Actor|DestroyActor))

(event EventBeginPlay
  (bind _outactors (Actor|GetAllActorsOfClass "/Game/Spyro_Run/PowerUps/PowerupManager.PowerupManager_C"))
  (bind _aspowerup_manager (Utilities|Casting|CastToPowerupManager (Utilities|Array|Get(acopy) _outactors)))
  (Variables|Default|SetPowerupManager _aspowerup_manager))

(event EventTick
  (params (DeltaSeconds :type Float%20%28single-precision%29))
  (if (Variables|Default|GetPickedUp?)
    (Variables|/Script/Engine.CharacterMovementComponent|SetMaxWalkSpeed (Variables|/Script/Engine.Character|GetCharacterMovement (Game|GetPlayerCharacter 0)) 1.2e+03)))

(fn ConstructionScript)