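; Base track tile for the Spyro Run runner, which reports itself to the TileManager and triggers spawning as the player advances.
; Its construction script sets the manager's next spawn point from NextSpawnLocation, and BeginPlay passes on its direction and bridge flag.
; When the player character overlaps its Box, it calls SpawnTiles on the manager and sends PassedPlatformMessage to every BI_Runner actor.
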(event OnComponentBeginOverlap(Box)
  (params (OverlappedComponent :type Primitive%20Component%20Object%20Reference) (OtherActor :type Actor%20Object%20Reference) (OtherComp :type Primitive%20Component%20Object%20Reference) (OtherBodyIndex :type Integer) (bFromSweep :type Boolean) (SweepResult :type Hit%20Result%20Structure%20%28by%20ref%29))
  (if (== OtherActor (Game|GetPlayerCharacter 0))
    (bind _outactors (Actor|GetAllActorsOfClass "/Game/Spyro_Run/Tiles/TileManager.TileManager_C"))
    (bind _astile_manager (Utilities|Casting|CastToTileManager (Utilities|Array|Get(acopy) _outactors)))
    (Default|SpawnTiles _astile_manager)
    (bind _outactors_2 (Actor|GetAllActorswithInterface "/Game/Spyro_Run/BI_Runner.BI_Runner_C"))
    (for _array_element _outactors_2
      (Class|BIRunner|PassedPlatform(Message) _array_element))))

(event EventBeginPlay
  (bind _outactors (Actor|GetAllActorsOfClass "/Game/Spyro_Run/Tiles/TileManager.TileManager_C"))
  (bind _astile_manager (Utilities|Casting|CastToTileManager (Utilities|Array|Get(acopy) _outactors)))
  (Variables|/Game/Spyro_Run/Tiles/TileManager.TileManager_C|SetTileDirection _astile_manager (Variables|Default|GetDirection))
  (Variables|/Game/Spyro_Run/Tiles/TileManager.TileManager_C|SetIsABridge? _astile_manager (Variables|Default|GetIsABridge?)))

(fn ConstructionScript
  (bind _outactors (Actor|GetAllActorsOfClass "/Game/Spyro_Run/Tiles/TileManager.TileManager_C"))
  (bind _astile_manager (Utilities|Casting|CastToTileManager (Utilities|Array|Get(acopy) _outactors)))
  (Variables|/Game/Spyro_Run/Tiles/TileManager.TileManager_C|SetNextSpawn _astile_manager (Transformation|GetWorldLocation (Variables|Default|GetNextSpawnLocation))))